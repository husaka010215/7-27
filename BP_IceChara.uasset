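; Player character for a timed ice-collecting game, with world-axis movement, look input and a pause menu.
; Overlapping a BP_Ice always spawns a BP_TuikaIce on the first mesh socket, then checks BP_GameInstance.IceItem1P to attach another at the socket numbered for that count, up to fifteen.
; A Delay on Tick drives a countdown that shows WBP_Finish, pauses and opens the "score" level once below zero.
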(event `InputAxis|MoveForwed`
  (params (AxisValue :type "Float (single-precision)"))
  (`self.AddMovementInput` (1.0 0.0 0.0) AxisValue))

(event `InputAxis|LookUp`
  (params (AxisValue :type "Float (single-precision)"))
  (`self.AddControllerPitchInput` AxisValue))

(event `InputAxis|LookRight`
  (params (AxisValue :type "Float (single-precision)"))
  (`self.AddControllerYawInput` AxisValue))

(event `InputAxis|MoveRight`
  (params (AxisValue :type "Float (single-precision)"))
  (`self.AddMovementInput` (0.0 1.0 0.0) AxisValue))

(event `self.ReceiveTick`
  (params (DeltaSeconds :type "Float (single-precision)"))
  (`KismetSystemLibrary.Delay` 1.0)
  (bind _output_get (set `self.Seconds` (- (`self.Seconds`) 1)))
  (`KismetSystemLibrary.PrintString` (`KismetStringLibrary.Conv_IntToString` _output_get))
  (if (< (`self.Seconds`) 0)
    (`WidgetLayoutLibrary.RemoveAllWidgets`)
    (bind _returnvalue (`|CreateWidget` "/Game/IceCatch/UIまとめ/WBP_Finish.WBP_Finish_C"))
    (`UserWidget.AddToViewport` _returnvalue 0)
    (set `PlayerController.bShowMouseCursor` false (`GameplayStatics.GetPlayerController` 0))
    (`GameplayStatics.SetGamePaused` true)
    ;[1 1 1] エンド画面を別に用意して、そこのレベルブループリントにウィジェット作成すればいいじゃ
    (`GameplayStatics.OpenLevel` "score")))

(event `InputAction|Pause`
  (params (Key :type "Key Structure"))
  (bind _returnvalue (`GameplayStatics.GetPlayerController` 0))
  (:`Pressed`
    (`WidgetLayoutLibrary.RemoveAllWidgets`)
    (bind _returnvalue_2 (`|CreateWidget` "/Game/IceCatch/UIまとめ/WBP_Pause.WBP_Pause_C"))
    (`UserWidget.AddToViewport` _returnvalue_2 0)
    (set `PlayerController.bShowMouseCursor` true _returnvalue)
    (`WidgetBlueprintLibrary.SetInputMode_UIOnlyEx` _returnvalue null) ; UI用のモードに切り替える
    ;[0.3886 1 0.7649] できた！！多分！！！
    (`GameplayStatics.SetGamePaused` true)))

(event `self.CapsuleComponent.OnComponentBeginOverlap`
  (params (OverlappedComponent :type "PrimitiveComponent Object Reference") (OtherActor :type "Actor Object Reference") (OtherComp :type "PrimitiveComponent Object Reference") (OtherBodyIndex :type Integer) (bFromSweep :type Boolean) (SweepResult :type "HitResult Structure (by ref)"))
  (cast `/Game/IceCatch/BP_Ice` OtherActor)
  (`|ExecutionSequence`
    (:`then_0`
      (`KismetSystemLibrary.PrintString` "できたわ。")
      (bind _returnvalue (`|SpawnActorFromClass` "/Game/IceCatch/BP_TuikaIce.BP_TuikaIce_C" (`SceneComponent.GetSocketTransform` (`self.Mesh`) "Iceソケット" "RTS_World") "Undefined" "OverrideRootScale" null null))
      (`self.K2_AttachToComponent` _returnvalue (`self.Mesh`) "Iceソケット" "SnapToTarget" "SnapToTarget" "SnapToTarget" true))
    (:`then_1`
      ;[1 0.1 0.7705] 2個なら2個目作る
      (if (== (`/Game/IceCatch/BP_GameInstance.IceItem_1P` (cast `/Game/IceCatch/BP_GameInstance` (`GameplayStatics.GetGameInstance`) :!pure true)) 2)
        (`KismetSystemLibrary.PrintString` "どう？")
        (bind _returnvalue_2 (`|SpawnActorFromClass` "/Game/IceCatch/BP_TuikaIce.BP_TuikaIce_C" (`SceneComponent.GetSocketTransform` (`self.Mesh`) "Iceソケット2" "RTS_World") "Undefined" "OverrideRootScale" null null))
        (`self.K2_AttachToComponent` _returnvalue_2 (`self.Mesh`) "Iceソケット2" "SnapToTarget" "SnapToTarget" "SnapToTarget" true)))
    (:`then_2`
      (if (== (`/Game/IceCatch/BP_GameInstance.IceItem_1P` (cast `/Game/IceCatch/BP_GameInstance` (`GameplayStatics.GetGameInstance`) :!pure true)) 3)
        (bind _returnvalue_3 (`|SpawnActorFromClass` "/Game/IceCatch/BP_TuikaIce.BP_TuikaIce_C" (`SceneComponent.GetSocketTransform` (`self.Mesh`) "Iceソケット3" "RTS_World") "Undefined" "OverrideRootScale" null null))
        (`self.K2_AttachToComponent` _returnvalue_3 (`self.Mesh`) "Iceソケット3" "SnapToTarget" "SnapToTarget" "SnapToTarget" true)))
    (:`then_3`
      (if (== (`/Game/IceCatch/BP_GameInstance.IceItem_1P` (cast `/Game/IceCatch/BP_GameInstance` (`GameplayStatics.GetGameInstance`) :!pure true)) 4)
        (bind _returnvalue_4 (`|SpawnActorFromClass` "/Game/IceCatch/BP_TuikaIce.BP_TuikaIce_C" (`SceneComponent.GetSocketTransform` (`self.Mesh`) "Iceソケット4" "RTS_World") "Undefined" "OverrideRootScale" null null))
        (`self.K2_AttachToComponent` _returnvalue_4 (`self.Mesh`) "Iceソケット4" "SnapToTarget" "SnapToTarget" "SnapToTarget" true)))
    (:`then_4`
      (if (== (`/Game/IceCatch/BP_GameInstance.IceItem_1P` (cast `/Game/IceCatch/BP_GameInstance` (`GameplayStatics.GetGameInstance`) :!pure true)) 5)
        (bind _returnvalue_5 (`|SpawnActorFromClass` "/Game/IceCatch/BP_TuikaIce.BP_TuikaIce_C" (`SceneComponent.GetSocketTransform` (`self.Mesh`) "Iceソケット5" "RTS_World") "Undefined" "OverrideRootScale" null null))
        (`self.K2_AttachToComponent` _returnvalue_5 (`self.Mesh`) "Iceソケット5" "SnapToTarget" "SnapToTarget" "SnapToTarget" true)))
    (:`then_5`
      (if (== (`/Game/IceCatch/BP_GameInstance.IceItem_1P` (cast `/Game/IceCatch/BP_GameInstance` (`GameplayStatics.GetGameInstance`) :!pure true)) 6)
        (bind _returnvalue_6 (`|SpawnActorFromClass` "/Game/IceCatch/BP_TuikaIce.BP_TuikaIce_C" (`SceneComponent.GetSocketTransform` (`self.Mesh`) "Iceソケット6" "RTS_World") "Undefined" "OverrideRootScale" null null))
        (`self.K2_AttachToComponent` _returnvalue_6 (`self.Mesh`) "Iceソケット6" "SnapToTarget" "SnapToTarget" "SnapToTarget" true)))
    (:`then_6`
      (if (== (`/Game/IceCatch/BP_GameInstance.IceItem_1P` (cast `/Game/IceCatch/BP_GameInstance` (`GameplayStatics.GetGameInstance`) :!pure true)) 7)
        (bind _returnvalue_7 (`|SpawnActorFromClass` "/Game/IceCatch/BP_TuikaIce.BP_TuikaIce_C" (`SceneComponent.GetSocketTransform` (`self.Mesh`) "Iceソケット7" "RTS_World") "Undefined" "OverrideRootScale" null null))
        (`self.K2_AttachToComponent` _returnvalue_7 (`self.Mesh`) "Iceソケット7" "SnapToTarget" "SnapToTarget" "SnapToTarget" true)))
    (:`then_7`
      (if (== (`/Game/IceCatch/BP_GameInstance.IceItem_1P` (cast `/Game/IceCatch/BP_GameInstance` (`GameplayStatics.GetGameInstance`) :!pure true)) 8)
        (bind _returnvalue_8 (`|SpawnActorFromClass` "/Game/IceCatch/BP_TuikaIce.BP_TuikaIce_C" (`SceneComponent.GetSocketTransform` (`self.Mesh`) "Iceソケット8" "RTS_World") "Undefined" "OverrideRootScale" null null))
        (`self.K2_AttachToComponent` _returnvalue_8 (`self.Mesh`) "Iceソケット8" "SnapToTarget" "SnapToTarget" "SnapToTarget" true)))
    (:`then_8`
      (if (== (`/Game/IceCatch/BP_GameInstance.IceItem_1P` (cast `/Game/IceCatch/BP_GameInstance` (`GameplayStatics.GetGameInstance`) :!pure true)) 9)
        (bind _returnvalue_9 (`|SpawnActorFromClass` "/Game/IceCatch/BP_TuikaIce.BP_TuikaIce_C" (`SceneComponent.GetSocketTransform` (`self.Mesh`) "Iceソケット9" "RTS_World") "Undefined" "OverrideRootScale" null null))
        (`self.K2_AttachToComponent` _returnvalue_9 (`self.Mesh`) "Iceソケット9" "SnapToTarget" "SnapToTarget" "SnapToTarget" true)))
    (:`then_9`
      (if (== (`/Game/IceCatch/BP_GameInstance.IceItem_1P` (cast `/Game/IceCatch/BP_GameInstance` (`GameplayStatics.GetGameInstance`) :!pure true)) 10)
        (bind _returnvalue_10 (`|SpawnActorFromClass` "/Game/IceCatch/BP_TuikaIce.BP_TuikaIce_C" (`SceneComponent.GetSocketTransform` (`self.Mesh`) "Iceソケット10" "RTS_World") "Undefined" "OverrideRootScale" null null))
        (`self.K2_AttachToComponent` _returnvalue_10 (`self.Mesh`) "Iceソケット10" "SnapToTarget" "SnapToTarget" "SnapToTarget" true)))
    (:`then_10`
      (if (== (`/Game/IceCatch/BP_GameInstance.IceItem_1P` (cast `/Game/IceCatch/BP_GameInstance` (`GameplayStatics.GetGameInstance`) :!pure true)) 11)
        (bind _returnvalue_11 (`|SpawnActorFromClass` "/Game/IceCatch/BP_TuikaIce.BP_TuikaIce_C" (`SceneComponent.GetSocketTransform` (`self.Mesh`) "Iceソケット11" "RTS_World") "Undefined" "OverrideRootScale" null null))
        (`self.K2_AttachToComponent` _returnvalue_11 (`self.Mesh`) "Iceソケット11" "SnapToTarget" "SnapToTarget" "SnapToTarget" true)))
    (:`then_11`
      (if (== (`/Game/IceCatch/BP_GameInstance.IceItem_1P` (cast `/Game/IceCatch/BP_GameInstance` (`GameplayStatics.GetGameInstance`) :!pure true)) 12)
        (bind _returnvalue_12 (`|SpawnActorFromClass` "/Game/IceCatch/BP_TuikaIce.BP_TuikaIce_C" (`SceneComponent.GetSocketTransform` (`self.Mesh`) "Iceソケット12" "RTS_World") "Undefined" "OverrideRootScale" null null))
        (`self.K2_AttachToComponent` _returnvalue_12 (`self.Mesh`) "Iceソケット12" "SnapToTarget" "SnapToTarget" "SnapToTarget" true)))
    (:`then_12`
      (if (== (`/Game/IceCatch/BP_GameInstance.IceItem_1P` (cast `/Game/IceCatch/BP_GameInstance` (`GameplayStatics.GetGameInstance`) :!pure true)) 13)
        (bind _returnvalue_13 (`|SpawnActorFromClass` "/Game/IceCatch/BP_TuikaIce.BP_TuikaIce_C" (`SceneComponent.GetSocketTransform` (`self.Mesh`) "Iceソケット13" "RTS_World") "Undefined" "OverrideRootScale" null null))
        (`self.K2_AttachToComponent` _returnvalue_13 (`self.Mesh`) "Iceソケット13" "SnapToTarget" "SnapToTarget" "SnapToTarget" true)))
    (:`then_13`
      (if (== (`/Game/IceCatch/BP_GameInstance.IceItem_1P` (cast `/Game/IceCatch/BP_GameInstance` (`GameplayStatics.GetGameInstance`) :!pure true)) 14)
        (bind _returnvalue_14 (`|SpawnActorFromClass` "/Game/IceCatch/BP_TuikaIce.BP_TuikaIce_C" (`SceneComponent.GetSocketTransform` (`self.Mesh`) "Iceソケット14" "RTS_World") "Undefined" "OverrideRootScale" null null))
        (`self.K2_AttachToComponent` _returnvalue_14 (`self.Mesh`) "Iceソケット14" "SnapToTarget" "SnapToTarget" "SnapToTarget" true)))
    (:`then_14`
      (if (== (`/Game/IceCatch/BP_GameInstance.IceItem_1P` (cast `/Game/IceCatch/BP_GameInstance` (`GameplayStatics.GetGameInstance`) :!pure true)) 15)
        (bind _returnvalue_15 (`|SpawnActorFromClass` "/Game/IceCatch/BP_TuikaIce.BP_TuikaIce_C" (`SceneComponent.GetSocketTransform` (`self.Mesh`) "Iceソケット15" "RTS_World") "Undefined" "OverrideRootScale" null null))
        (`self.K2_AttachToComponent` _returnvalue_15 (`self.Mesh`) "Iceソケット15" "SnapToTarget" "SnapToTarget" "SnapToTarget" true)))))

(fn `UserConstructionScript`)